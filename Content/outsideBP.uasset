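; Debug actor that tests whether the player camera's view lines up with this actor, apparently to detect looking outside.
; Every Tick, it dots the actor-to-camera direction with the camera's forward vector after a 180-degree rotation, then negates the result.
; A fixed threshold on that value selects between printing "Looking outside" and "NOT", with no other gameplay effect.
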(event `self.ReceiveTick`
  (params (DeltaSeconds :type "Float (single-precision)"))
  (bind _returnvalue (`GameplayStatics.GetPlayerCameraManager` 0))
  (if (< (* (`KismetMathLibrary.Dot_VectorVector` (`KismetMathLibrary.GetForwardVector` (`KismetMathLibrary.FindLookAtRotation` (`self.K2_GetActorLocation`) (`PlayerCameraManager.GetCameraLocation` _returnvalue))) (`KismetMathLibrary.GreaterGreater_VectorRotator` (`KismetMathLibrary.GetForwardVector` (`PlayerCameraManager.GetCameraRotation` _returnvalue)) (struct :`Yaw` -180.0))) -1.0) -0.9)
    (`KismetSystemLibrary.PrintString` "Looking outside")
    (else
      (`KismetSystemLibrary.PrintString` "NOT"))))

(fn `UserConstructionScript`)